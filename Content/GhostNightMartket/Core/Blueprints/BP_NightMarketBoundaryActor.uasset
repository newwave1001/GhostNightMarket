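; Night market boundary volume that starts and ends relic exploration as the player character crosses its box.
; On entry, it sets an exploring flag, guarded against repeat triggers, and tells every relic spot manager in the level to spawn relics.
; On exit, it clears the flag, marks every relic spot as collected and calls hide-in-game on itself within that loop, rather than on the spots.
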(event OnComponentBeginOverlap(Box)
  (params (OverlappedComponent :type Primitive%20Component%20Object%20Reference) (OtherActor :type Actor%20Object%20Reference) (OtherComp :type Primitive%20Component%20Object%20Reference) (OtherBodyIndex :type Integer) (bFromSweep :type Boolean) (SweepResult :type Hit%20Result%20Structure%20%28by%20ref%29))
  (Utilities|Casting|CastToBP_ThirdPersonCharacter OtherActor)
  (if (== (Variables|Default|GetIsExploring) false)
    (Variables|Default|SetIsExploring true)
    (bind _outactors (Actor|GetAllActorsOfClass "/Game/GhostNightMartket/Core/Blueprints/BP_RelicSpotManagerActor.BP_RelicSpotManagerActor_C"))
    (for _array_element _outactors
      (Default|SpawnRelics _array_element))))

(event OnComponentEndOverlap(Box)
  (params (OverlappedComponent :type Primitive%20Component%20Object%20Reference) (OtherActor :type Actor%20Object%20Reference) (OtherComp :type Primitive%20Component%20Object%20Reference) (OtherBodyIndex :type Integer))
  (Utilities|Casting|CastToBP_ThirdPersonCharacter OtherActor)
  (Variables|Default|SetIsExploring false)
  (bind _outactors (Actor|GetAllActorsOfClass "/Game/GhostNightMartket/Core/Blueprints/BP_RelicSpot.BP_RelicSpot_C"))
  (for _array_element _outactors
    (Variables|/Game/GhostNightMartket/Core/Blueprints/BP_RelicSpot.BP_RelicSpot_C|SetIsCollected _array_element true)
    (Rendering|SetActorHiddenInGame true)))

(fn ConstructionScript)