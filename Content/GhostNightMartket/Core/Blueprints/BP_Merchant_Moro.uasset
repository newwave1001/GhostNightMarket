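; BP_Merchant_Moro is the merchant Moro, whose only active logic is Open Shop, which puts the player into a pawn shop screen.
; It hides its widget and the player character, blends the view to itself, and switches to UI-only input with a cursor.
; It then clears the Game Instance inventory, has the first BP_NightMarketManager found initialize the shop, and adds a new W_PawnShopUI to the viewport.
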(event EventBeginPlay
  (|CallParentFunction) ; This node is disabled and will not be called.\nDrag off pins to build functionality.
)

(event Collision|EventActorBeginOverlap
  (params (OtherActor :type Actor%20Object%20Reference))
  (|CallParentFunction OtherActor) ; This node is disabled and will not be called.\nDrag off pins to build functionality.
)

(event EventTick
  (params (DeltaSeconds :type Float%20%28single-precision%29))
  (|CallParentFunction DeltaSeconds) ; This node is disabled and will not be called.\nDrag off pins to build functionality.
)

(fn ConstructionScript
  (|CallParentFunction))

(fn OpenShop
  (bind _returnvalue (Game|GetPlayerController 0))
  (Rendering|SetVisibility (Variables|Default|GetWidget) false false)
  (Game|Player|SetViewTargetwithBlend _returnvalue self 0.3 "VTBlend_Linear" 0.0 true)
  (Input|SetInputModeUIOnly _returnvalue (Variables|Default|GetShopWidget) "DoNotLock" false)
  (Variables|/Script/Engine.PlayerController|SetbShowMouseCursor _returnvalue true)
  (Rendering|SetActorHiddenInGame (Game|GetPlayerCharacter 0) true)
  (bind _asbp_game_instance (Utilities|Casting|CastToBP_GameInstance (Game|GetGameInstance)))
  (Utilities|Array|Clear (Variables|/Game/GhostNightMartket/Core/Blueprints/BP_GameInstance.BP_GameInstance_C|GetInventory _asbp_game_instance))
  (bind _outactors (Actor|GetAllActorsOfClass "/Game/GhostNightMartket/Core/Blueprints/BP_NightMarketManager.BP_NightMarketManager_C"))
  (Default|InitializedShop (Utilities|Array|Get(acopy) _outactors))
  (bind _returnvalue_2 (UserInterface|CreateWidget "/Game/GhostNightMartket/UI/Widgets/W_PawnShopUI.W_PawnShopUI_C"))
  (bind _output_get (Variables|Default|SetPawnShopWidget_0 _returnvalue_2))
  (UserInterface|Viewport|AddtoViewport _output_get 0))