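; BP_RelicSpotManagerActor is a placed spawner that scatters relic spots around its location when play begins.
; SpawnRelics creates SpawnCount BP_RelicSpot actors at random X/Y offsets within SpawnRadius, covering a square rather than a circle.
; Spawn Z is left unset rather than taken from the manager's height.
; The construction script sizes the RangeDisplay sphere to SpawnRadius to show the range.
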(event EventBeginPlay
  (CallFunction|SpawnRelics))

(event Collision|EventActorBeginOverlap
  (params (OtherActor :type Actor%20Object%20Reference)))

(event EventTick
  (params (DeltaSeconds :type Float%20%28single-precision%29)))

(fn ConstructionScript
  (Components|Sphere|SetSphereRadius (Variables|Default|GetRangeDisplay) (Variables|Default|GetSpawnRadius) true))

(fn SpawnRelics
  (bind _returnvalue (Transformation|GetActorLocation))
  (bind _spawnradius (Variables|Default|GetSpawnRadius))
  (bind _spawnradius_2 (Variables|Default|GetSpawnRadius))
  (bind _spawnradius_3 (Variables|Default|GetSpawnRadius))
  (bind _spawnradius_4 (Variables|Default|GetSpawnRadius))
  (bind _returnvalue_2 (* _spawnradius_2 -1.0))
  (bind _returnvalue_3 (* _spawnradius_3 -1.0))
  (bind _returnvalue_4 (Math|Random|RandomFloatinRange _returnvalue_2 _spawnradius))
  (bind _returnvalue_5 (Math|Random|RandomFloatinRange _returnvalue_3 _spawnradius_4))
  (bind _returnvalue_6 (Math|Vector|MakeVector _returnvalue_5 _returnvalue_4 0.0))
  (bind _returnvalue_7 (+ _returnvalue _returnvalue_6))
  (for _index (range 1 (Variables|Default|GetSpawnCount))
    (Game|SpawnActorfromClass "/Game/GhostNightMartket/Core/Blueprints/BP_RelicSpot.BP_RelicSpot_C" (Math|Transform|MakeTransform (Math|Vector|MakeVector (.x _returnvalue_7) (.y _returnvalue_7) 0.0) "0, 0, 0" "1.000000,1.000000,1.000000") "Undefined" "MultiplyWithRoot" 0 0)))