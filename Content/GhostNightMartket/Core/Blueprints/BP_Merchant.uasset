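; BP_Merchant is a night market merchant whose data loads from DT_Merchants by MerchantID.
; Its interaction sphere registers it as the player character's CurrentMerchant and toggles a widget on overlap.
; OpenShop blends the camera to the merchant, hides the player, clears the GameInstance inventory, initializes the shop through BP_NightMarketManager and adds shop and inventory UIs.
; CloseShop removes all widgets and restores player visibility, game input and camera.
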(event OnComponentBeginOverlap(InteractionSphere)
  (params (OverlappedComponent :type Primitive%20Component%20Object%20Reference) (OtherActor :type Actor%20Object%20Reference) (OtherComp :type Primitive%20Component%20Object%20Reference) (OtherBodyIndex :type Integer) (bFromSweep :type Boolean) (SweepResult :type Hit%20Result%20Structure%20%28by%20ref%29))
  (bind _asbp_third_person_character (Utilities|Casting|CastToBP_ThirdPersonCharacter OtherActor))
  (Utilities|IsValid _asbp_third_person_character
    (:Is%20Valid
      (Variables|/Game/ThirdPerson/Blueprints/BP_ThirdPersonCharacter.BP_ThirdPersonCharacter_C|SetCurrentMerchant _asbp_third_person_character self)
      (Rendering|SetVisibility (Variables|Default|GetWidget) true false))))

(event OnComponentEndOverlap(InteractionSphere)
  (params (OverlappedComponent :type Primitive%20Component%20Object%20Reference) (OtherActor :type Actor%20Object%20Reference) (OtherComp :type Primitive%20Component%20Object%20Reference) (OtherBodyIndex :type Integer))
  (bind _asbp_third_person_character (Utilities|Casting|CastToBP_ThirdPersonCharacter OtherActor))
  (Utilities|IsValid _asbp_third_person_character
    (:Is%20Valid
      (Variables|/Game/ThirdPerson/Blueprints/BP_ThirdPersonCharacter.BP_ThirdPersonCharacter_C|SetCurrentMerchant _asbp_third_person_character 0)
      (Rendering|SetVisibility (Variables|Default|GetWidget) false false))))

(event EventBeginPlay
  (CallFunction|LoadMerchantData))

(event Collision|EventActorBeginOverlap
  (params (OtherActor :type Actor%20Object%20Reference)))

(event EventTick
  (params (DeltaSeconds :type Float%20%28single-precision%29)))

(fn ConstructionScript)

(fn LoadMerchantData
  (bind _returnvalue (Utilities|GetDataTableRow "/Game/GhostNightMartket/Core/DataTables/DT_Merchants.DT_Merchants" (Variables|Default|GetMerchantID))
    (:then
      (Variables|Default|SetMerchantData _returnvalue))))

(fn OpenShop
  (bind _returnvalue (Game|GetPlayerController 0))
  (Variables|Default|SetShopWidget 0)
  (Variables|Default|SetInventoryWidget 0)
  (Rendering|SetVisibility (Variables|Default|GetWidget) false false)
  (Game|Player|SetViewTargetwithBlend _returnvalue self 0.3 "VTBlend_Linear" 0.0 true)
  (Input|SetInputModeUIOnly _returnvalue (Variables|Default|GetShopWidget) "DoNotLock" false)
  (Variables|/Script/Engine.PlayerController|SetbShowMouseCursor _returnvalue true)
  (Rendering|SetActorHiddenInGame (Game|GetPlayerCharacter 0) true)
  (bind _asbp_game_instance (Utilities|Casting|CastToBP_GameInstance (Game|GetGameInstance)))
  (Utilities|Array|Clear (Variables|/Game/GhostNightMartket/Core/Blueprints/BP_GameInstance.BP_GameInstance_C|GetInventory _asbp_game_instance))
  (bind _outactors (Actor|GetAllActorsOfClass "/Game/GhostNightMartket/Core/Blueprints/BP_NightMarketManager.BP_NightMarketManager_C"))
  (Default|InitializedShop (Utilities|Array|Get(acopy) _outactors))
  (bind _returnvalue_2 (UserInterface|CreateWidget "/Game/GhostNightMartket/UI/Widgets/W_NightMarketUI.W_NightMarketUI_C"))
  (Variables|Default|SetShopWidget _returnvalue_2)
  (Default|SetMerchantData (Variables|Default|GetShopWidget) (Variables|Default|GetMerchantData))
  (UserInterface|Viewport|AddtoViewport _returnvalue_2 0)
  (bind _returnvalue_3 (UserInterface|CreateWidget "/Game/GhostNightMartket/UI/Widgets/W_InventoryUI.W_InventoryUI_C"))
  (bind _output_get (Variables|Default|SetInventoryWidget _returnvalue_3))
  (UserInterface|Viewport|AddtoViewport _output_get 0))

(fn CloseShop
  (bind _returnvalue (Game|GetPlayerCharacter 0))
  (bind _returnvalue_2 (Game|GetPlayerController 0))
  (Viewport|RemoveAllWidgets)
  (Rendering|SetActorHiddenInGame _returnvalue false)
  (Input|SetInputModeGameOnly _returnvalue_2 false)
  (Variables|/Script/Engine.PlayerController|SetbShowMouseCursor _returnvalue_2 false)
  (Game|Player|SetViewTargetwithBlend _returnvalue_2 _returnvalue 0.3 "VTBlend_Linear" 0.0 false))