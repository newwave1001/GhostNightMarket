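; Relic pickup spot that holds a random wild-spawnable item from DT_Items, chosen at BeginPlay.
; Overlap volumes reveal discovery effects, toggle the prompt widget and register the spot as the player's CurrentRelicSpot.
; OpenCompassMinigame shows a notification if the inventory is full, otherwise opens compass and inventory widgets, scaling minigame difficulty by rarity.
; SpawnWindEffect, called by a timer, and ClosedGame are empty stubs.
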(event OnComponentBeginOverlap(DetectionRange)
  (params (OverlappedComponent :type Primitive%20Component%20Object%20Reference) (OtherActor :type Actor%20Object%20Reference) (OtherComp :type Primitive%20Component%20Object%20Reference) (OtherBodyIndex :type Integer) (bFromSweep :type Boolean) (SweepResult :type Hit%20Result%20Structure%20%28by%20ref%29))
  (Utilities|Casting|CastToBP_ThirdPersonCharacter OtherActor)
  (if (not (Variables|Default|GetIsCollected))
    (Rendering|SetVisibility (Variables|Default|GetDiscoveryEffect) true false)
    (Components|Activation|Activate (Variables|Default|GetRelicEffec) false)))

(event OnComponentEndOverlap(DetectionRange)
  (params (OverlappedComponent :type Primitive%20Component%20Object%20Reference) (OtherActor :type Actor%20Object%20Reference) (OtherComp :type Primitive%20Component%20Object%20Reference) (OtherBodyIndex :type Integer))
  (Utilities|Casting|CastToBP_ThirdPersonCharacter OtherActor)
  (if (not (Variables|Default|GetIsCollected))
    (Rendering|SetVisibility (Variables|Default|GetDiscoveryEffect) false false)
    (Components|Activation|Deactivate (Variables|Default|GetRelicEffec))))

(event OnComponentBeginOverlap(InteractionRange)
  (params (OverlappedComponent :type Primitive%20Component%20Object%20Reference) (OtherActor :type Actor%20Object%20Reference) (OtherComp :type Primitive%20Component%20Object%20Reference) (OtherBodyIndex :type Integer) (bFromSweep :type Boolean) (SweepResult :type Hit%20Result%20Structure%20%28by%20ref%29))
  (bind _asbp_third_person_character (Utilities|Casting|CastToBP_ThirdPersonCharacter OtherActor))
  (Utilities|IsValid _asbp_third_person_character
    (:Is%20Valid
      (Variables|/Game/ThirdPerson/Blueprints/BP_ThirdPersonCharacter.BP_ThirdPersonCharacter_C|SetCurrentRelicSpot _asbp_third_person_character self)
      (Rendering|SetVisibility (Variables|Default|GetWidget) true false))))

(event OnComponentEndOverlap(InteractionRange)
  (params (OverlappedComponent :type Primitive%20Component%20Object%20Reference) (OtherActor :type Actor%20Object%20Reference) (OtherComp :type Primitive%20Component%20Object%20Reference) (OtherBodyIndex :type Integer))
  (bind _asbp_third_person_character (Utilities|Casting|CastToBP_ThirdPersonCharacter OtherActor))
  (if (== (Variables|/Game/ThirdPerson/Blueprints/BP_ThirdPersonCharacter.BP_ThirdPersonCharacter_C|GetCurrentRelicSpot _asbp_third_person_character) self)
    (Variables|/Game/ThirdPerson/Blueprints/BP_ThirdPersonCharacter.BP_ThirdPersonCharacter_C|SetCurrentRelicSpot _asbp_third_person_character 0)
    (Rendering|SetVisibility (Variables|Default|GetWidget) false false)))

(event OnComponentBeginOverlap(DetectionRange1)
  (params (OverlappedComponent :type Primitive%20Component%20Object%20Reference) (OtherActor :type Actor%20Object%20Reference) (OtherComp :type Primitive%20Component%20Object%20Reference) (OtherBodyIndex :type Integer) (bFromSweep :type Boolean) (SweepResult :type Hit%20Result%20Structure%20%28by%20ref%29))
  (Utilities|Time|SetTimerbyFunctionName 0 "SpawnWindEffect" 3.0 true))

(event OnComponentEndOverlap(DetectionRange1)
  (params (OverlappedComponent :type Primitive%20Component%20Object%20Reference) (OtherActor :type Actor%20Object%20Reference) (OtherComp :type Primitive%20Component%20Object%20Reference) (OtherBodyIndex :type Integer))
  (Utilities|Time|SetTimerbyFunctionName 0 "SpawnWindEffect" 3.0))

(event EventBeginPlay
  (bind _validitems (Variables|Default|GetValidItems))
  (bind _validitems_2 (Variables|Default|GetValidItems))
  (bind _returnvalue (Utilities|Array|Length _validitems))
  (bind _returnvalue_2 (- _returnvalue -1))
  (bind _returnvalue_3 (Math|Random|RandomIntegerinRange 0 _returnvalue_2))
  (bind _output (Utilities|Array|Get(acopy) _validitems_2 _returnvalue_3))
  (Utilities|Array|Clear (Variables|Default|GetValidItems))
  (bind _outrownames (DataTable|GetDataTableRowNames "/Game/GhostNightMartket/Core/DataTables/DT_Items.DT_Items"))
  (for _array_element _outrownames
    (bind _returnvalue_4 (Utilities|GetDataTableRow "/Game/GhostNightMartket/Core/DataTables/DT_Items.DT_Items" _array_element)
      (:then
        (if (.CanSpawnInWild (Utilities|Struct|BreakFItemData _returnvalue_4))
          (Utilities|Array|Add _validitems_2 _returnvalue_4)
          (if (> (Utilities|Array|Length (Variables|Default|GetValidItems)) 0)
            (Variables|Default|SetRelicItem _output)
            (else
              (Actor|DestroyActor)))))))
  (Variables|Default|SetRelicItem _output))

(event Collision|EventActorBeginOverlap
  (params (OtherActor :type Actor%20Object%20Reference)))

(event EventTick
  (params (DeltaSeconds :type Float%20%28single-precision%29)))

(fn ConstructionScript)

(fn OpenCompassMinigame
  (bind _returnvalue (Game|GetPlayerController 0))
  (bind _returnvalue_2 (Game|GetPlayerController 0))
  (bind _asbp_game_instance (Utilities|Casting|CastToBP_GameInstance (Game|GetGameInstance)))
  (if (>= (Utilities|Array|Length (Variables|/Game/GhostNightMartket/Core/Blueprints/BP_GameInstance.BP_GameInstance_C|GetInventory _asbp_game_instance)) (Variables|/Game/GhostNightMartket/Core/Blueprints/BP_GameInstance.BP_GameInstance_C|GetMaxInventorySlots _asbp_game_instance))
    ;[0.15 0.15 0.15 0.5] 인벤토리 꽉참
    (bind _returnvalue_3 (UserInterface|CreateWidget "/Game/GhostNightMartket/UI/Widgets/W_NotificationUI.W_NotificationUI_C"))
    (UserInterface|Viewport|AddtoViewport _returnvalue_3 0)
    (else
      (Input|SetInputModeUIOnly _returnvalue (Variables|Default|GetCompassWidget) "DoNotLock" false)
      (Variables|/Script/Engine.PlayerController|SetbShowMouseCursor _returnvalue true)
      (bind _returnvalue_4 (UserInterface|CreateWidget "/Game/GhostNightMartket/UI/Widgets/W_InventoryUI.W_InventoryUI_C"))
      (Default|RefreshInventory _returnvalue_4)
      (bind _returnvalue_5 (UserInterface|CreateWidget "/Game/GhostNightMartket/UI/Widgets/W_CompassMinigame.W_CompassMinigame_C"))
      (Variables|/Game/GhostNightMartket/UI/Widgets/W_CompassMinigame.W_CompassMinigame_C|SetOwnerRelicSpot _returnvalue_5 self)
      (Variables|/Game/GhostNightMartket/UI/Widgets/W_CompassMinigame.W_CompassMinigame_C|SetRelicItem _returnvalue_5 (Variables|Default|GetRelicItem))
      (Variables|/Game/GhostNightMartket/UI/Widgets/W_CompassMinigame.W_CompassMinigame_C|SetRequiredScore _returnvalue_5 (+ (* (.rarity (Variables|Default|GetRelicItem)) 10) 50))
      (Variables|/Game/GhostNightMartket/UI/Widgets/W_CompassMinigame.W_CompassMinigame_C|SetMaxClicks _returnvalue_5 (+ (.rarity (Variables|Default|GetRelicItem)) 7))
      (switch int (.Rarity (Utilities|Struct|BreakFItemData (Variables|Default|GetRelicItem)))
        (:1
          (Variables|/Game/GhostNightMartket/UI/Widgets/W_CompassMinigame.W_CompassMinigame_C|SetRotationSpeed _returnvalue_5 1.0))
        (:2
          (Variables|/Game/GhostNightMartket/UI/Widgets/W_CompassMinigame.W_CompassMinigame_C|SetRotationSpeed _returnvalue_5 1.5))
        (:3
          (Variables|/Game/GhostNightMartket/UI/Widgets/W_CompassMinigame.W_CompassMinigame_C|SetRotationSpeed _returnvalue_5 2.0))
        (:4
          (Variables|/Game/GhostNightMartket/UI/Widgets/W_CompassMinigame.W_CompassMinigame_C|SetRotationSpeed _returnvalue_5 2.5))
        (:5
          (Variables|/Game/GhostNightMartket/UI/Widgets/W_CompassMinigame.W_CompassMinigame_C|SetRotationSpeed _returnvalue_5 3.0)))
      (bind _asbp_third_person_character (Utilities|Casting|CastToBP_ThirdPersonCharacter (Game|GetPlayerCharacter 0)))
      (Default|SetCompassWidget _asbp_third_person_character)
      (bind _output_get (Variables|Default|SetCompassWidget _returnvalue_5))
      (UserInterface|Viewport|AddtoViewport _output_get 0)
      (Input|SetInputModeGameandUI _returnvalue_2 0 "DoNotLock" true false)
      (Variables|/Script/Engine.PlayerController|SetbShowMouseCursor _returnvalue_2 true))))

(fn SpawnWindEffect)

(fn ClosedGame)