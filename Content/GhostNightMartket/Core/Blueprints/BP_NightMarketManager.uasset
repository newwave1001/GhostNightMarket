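; Night market manager that builds the shop's stock and handles buying and selling against the GameInstance's money and inventory.
; InitializedShop rolls each DT_Items row for stock, with higher rarity raising the odds and curse tier lowering them, and randomizes prices around BasePrice.
; Its seeded RandomStream goes unused by these rolls, and ShopPrices is never cleared.
; BuyItem copies affordable stock into runtime items; SellItem pays BasePrice times ValueMultiplier.
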(event EventBeginPlay)

(event Collision|EventActorBeginOverlap
  (params (OtherActor :type Actor%20Object%20Reference)))

(event EventTick
  (params (DeltaSeconds :type Float%20%28single-precision%29)))

(fn ConstructionScript)

(fn InitializedShop
  (bind _asbp_game_instance (Utilities|Casting|CastToBP_GameInstance (Game|GetGameInstance)))
  (Variables|Default|SetRandomStream (Math|Random|MakeRandomStream (Variables|/Game/GhostNightMartket/Core/Blueprints/BP_GameInstance.BP_GameInstance_C|GetRandomSeed _asbp_game_instance)))
  (Utilities|Array|Clear (Variables|Default|GetShopInventory))
  (bind _outrownames (DataTable|GetDataTableRowNames "/Game/GhostNightMartket/Core/DataTables/DT_Items.DT_Items"))
  (for _array_element _outrownames
    (bind _returnvalue (Utilities|GetDataTableRow "/Game/GhostNightMartket/Core/DataTables/DT_Items.DT_Items" _array_element)
      (:then
        (if (<= (Math|Random|RandomFloatinRange 0.0 (Math|Conversions|ToFloat(Integer) (+ (- 100 (* (.Rarity (Utilities|Struct|BreakFItemData _returnvalue)) 15)) (* (.CurseTier (Utilities|Struct|BreakFItemData _returnvalue)) 5)))) 5e+01)
          (Utilities|Array|Add (Variables|Default|GetShopInventory) _returnvalue)
          (Utilities|Array|Add (Variables|Default|GetShopPrices) (Math|Float|Truncate (* (.BasePrice (Utilities|Struct|BreakFItemData _returnvalue)) (Math|Random|RandomFloatinRange 0.8 1.4)))))))))

(fn BuyItem
  (params (Index :type Integer))
  (bind _shopprices (Variables|Default|GetShopPrices))
  (bind _shopinventory (Variables|Default|GetShopInventory))
  (bind _output (Utilities|Array|Get(acopy) _shopprices Index))
  (bind _output_2 (Utilities|Array|Get(acopy) _shopinventory Index))
  (bind (_itemid _displayname _description _baseprice _rarity _cursetier _authenticity) (Utilities|Struct|BreakFItemData _output_2))
  (bind _asbp_game_instance (Utilities|Casting|CastToBP_GameInstance (Game|GetGameInstance)))
  (if (>= (Variables|/Game/GhostNightMartket/Core/Blueprints/BP_GameInstance.BP_GameInstance_C|GetMoney _asbp_game_instance) _output)
    (Variables|/Game/GhostNightMartket/Core/Blueprints/BP_GameInstance.BP_GameInstance_C|SetMoney _asbp_game_instance (- (Variables|/Game/GhostNightMartket/Core/Blueprints/BP_GameInstance.BP_GameInstance_C|GetMoney _asbp_game_instance) _output))
    (Utilities|Array|Add (Variables|/Game/GhostNightMartket/Core/Blueprints/BP_GameInstance.BP_GameInstance_C|GetInventory _asbp_game_instance) (Utilities|Struct|MakeFItemRuntime _itemid _displayname _baseprice 1.0 0.0 _rarity 0.0 false _cursetier _authenticity))))

(fn SellItem
  (params (Index :type Integer))
  (bind _asbp_game_instance (Utilities|Casting|CastToBP_GameInstance (Game|GetGameInstance)))
  (Variables|/Game/GhostNightMartket/Core/Blueprints/BP_GameInstance.BP_GameInstance_C|SetMoney _asbp_game_instance (+ (Variables|/Game/GhostNightMartket/Core/Blueprints/BP_GameInstance.BP_GameInstance_C|GetMoney _asbp_game_instance) (Math|Float|Truncate (* (.BasePrice (Utilities|Struct|BreakFItemRuntime (Utilities|Array|Get(acopy) (Variables|/Game/GhostNightMartket/Core/Blueprints/BP_GameInstance.BP_GameInstance_C|GetInventory _asbp_game_instance) Index))) (.ValueMultiplier (Utilities|Struct|BreakFItemRuntime (Utilities|Array|Get(acopy) (Variables|/Game/GhostNightMartket/Core/Blueprints/BP_GameInstance.BP_GameInstance_C|GetInventory _asbp_game_instance) Index)))))))
  (Utilities|Array|RemoveIndex (Variables|/Game/GhostNightMartket/Core/Blueprints/BP_GameInstance.BP_GameInstance_C|GetInventory _asbp_game_instance) Index))